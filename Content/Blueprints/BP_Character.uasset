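; Character Blueprint with a melee attack, health and an HP bar widget.
; BeginPlay creates the HP bar, assigns it to the widget component and sets HP to MaxHP.
; Attack plays one of three random montage sections, then immediately capsule-traces forward with debug drawing and applies fixed damage to the hit actor.
; AnyDamage subtracts HP and updates the bar; death is not handled and EndAttack is empty.
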(event Custom|Attack
  (bind _returnvalue (Transformation|GetActorLocation))
  ;[1 1 1] Attack
  (Animation|PlayAnimMontage "/Game/Animation/AM_Attack.AM_Attack" 1.0 (Utilities|String|StringToName (Utilities|String|ToString(Text) (Utilities|Text|FormatText "Attack_{index}" (Math|Random|RandomIntegerinRange 0 2)))))
  (bind (_outhit _returnvalue_2) (Collision|CapsuleTraceByChannel _returnvalue (+ _returnvalue (* (Transformation|GetActorForwardVector) (Variables|Default|GetAttackRange))) (Variables|Default|GetAttackRadius) (Variables|Default|GetAttackHeight) "TraceTypeQuery3" false 0 "ForDuration"))
  (if _returnvalue_2
    (Game|Damage|ApplyDamage (.HitActor (Collision|BreakHitResult _outhit)) 1e+01 0 0)))

(event Custom|EndAttack
  ;[1 1 1] End Attack
)

(event EventBeginPlay
  ;[1 1 1] Initialize
  (bind _returnvalue (UserInterface|CreateWidget "/Game/UI/WBP_HpBar.WBP_HpBar_C"))
  (bind _aswbp_hp_bar (Utilities|Casting|CastToWBP_HpBar _returnvalue))
  (bind _output_get (Variables|Default|SetHpBar _aswbp_hp_bar))
  (UserInterface|SetWidget (Variables|Default|GetHpBarWidget) _output_get)
  (Variables|Default|SetHP (Variables|Default|GetMaxHP)))

(event Game|Damage|EventAnyDamage
  (params (Damage :type Float%20%28single-precision%29) (DamageType :type Damage%20Type%20Object%20Reference) (InstigatedBy :type Controller%20Object%20Reference) (DamageCauser :type Actor%20Object%20Reference))
  (bind _output_get (Variables|Default|SetHP (- (Variables|Default|GetHP) Damage)))
  (Progress|SetPercent (Variables|/Game/UI/WBP_HpBar.WBP_HpBar_C|GetProgressHpBar (Variables|Default|GetHpBar)) (/ _output_get (Variables|Default|GetMaxHP))))

(fn ConstructionScript)